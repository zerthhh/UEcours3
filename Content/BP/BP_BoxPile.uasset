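; BP_BoxPile is a procedural prop that builds a randomized vertical pile of static meshes, such as boxes or books.
; The Construction Script loops BookCount times, adding a component with a random mesh from ObjectList at a random X/Y offset and yaw within set ranges.
; Each mesh's bounding-box height, scaled by a BoundingBox multiplier, accumulates into a running total that sets the stacking height.
; The event graph has no runtime logic.
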(fn `UserConstructionScript`
  (locals (CurrentStaticMesh :type "StaticMesh Object Reference") (CurrentObjectThickness :type "Float (double-precision)" :default 0.0) (`Current Total Objects Heght` :type "Float (double-precision)"))
  ;[1 1 1] Loop x Book Count
  (for _ (range 1 (+ (`self.Book Count`) 1))
    ;[1 1 1] Pick Random book from list
    (bind _output_get (set `local.CurrentStaticMesh` (`KismetArrayLibrary.Array_Random` (`self.Object List`))))
    (bind _returnvalue (`StaticMesh.GetBoundingBox` _output_get))
    (bind _output_get_2 (set `local.CurrentObjectThickness` (* (- (.z (`.Max` (break `Box` _returnvalue))) (.z (break `Box` _returnvalue))) (`self.Bounding Box`))))
    (bind _returnvalue_2 (`AddComponent|NODE_AddStaticMeshComponent-0` :`RelativeTransform` (`KismetMathLibrary.MakeTransform` (`KismetMathLibrary.MakeVector` (`KismetMathLibrary.RandomFloatInRange` (`self.Min translate X`) (`self.Max translate X`)) (`KismetMathLibrary.RandomFloatInRange` (`self.Min translate Y`) (`self.Max translate Y`)) (+ (`local.Current Total Objects Heght`) _output_get_2)) (`KismetMathLibrary.MakeRotator` 0.0 0.0 (`KismetMathLibrary.RandomFloatInRange` (`self.Min Rotation`) (`self.Max Rotation`))))))
    (`StaticMeshComponent.SetStaticMesh` _returnvalue_2 (`local.CurrentStaticMesh`))
    (set `local.Current Total Objects Heght` (+ (`local.CurrentObjectThickness`) (`local.Current Total Objects Heght`)))))